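; Behavior Tree node that scans for enemy targets on each AI tick, apparently unfinished since it never assigns a found target.
; It refreshes an ignore list, then sweeps a sphere trace forward from the controlled pawn.
; Each hit needs an unobstructed Camera-channel line trace and a dot-product check for the front hemisphere, but the result is only printed.
; With no hits, it sets the target blackboard key to an empty object.
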(event `self.ReceiveTickAI`
  (params (OwnerController :type "AIController Object Reference") (ControlledPawn :type "Pawn Object Reference") (DeltaSeconds :type "Float (single-precision)"))
  (`self.FindAllIgnoredObjects`)
  (bind (_hits _hitanything) (`self.SphereTest` ControlledPawn))
  (if _hitanything
    (for _array_element _hits
      (bind _success (`self.VisibilityTest` ControlledPawn (`.HitActor` (`GameplayStatics.BreakHitResult` _array_element))))
      (if _success
        (`KismetSystemLibrary.PrintString` "visible")
        (else
          (`KismetSystemLibrary.PrintString` "not visible"))))
    (else
      (`BTFunctionLibrary.SetBlackboardValueAsObject` (`self.TargetObjectKey`)))))

(fn `FindAllIgnoredObjects`
  (bind _outactors (`GameplayStatics.GetAllActorsOfClass` null))
  (set `self.Actors to Ignore` _outactors))

(fn `IsFacingTarget`
  (params (Skibidibi :type "Pawn Object Reference") (Bot :type "Actor Object Reference"))
  (returns (IsFacingTarget :type Boolean))
  (return (> (`KismetMathLibrary.Dot_VectorVector` (`Actor.GetActorForwardVector` Skibidibi) (`KismetMathLibrary.GetDirectionUnitVector` (`Actor.K2_GetActorLocation` Skibidibi) (`Actor.K2_GetActorLocation` Bot))) 0.0)))

(fn `SphereTest`
  (params (Skibidibi :type "Pawn Object Reference"))
  (returns (Hits :type "Array of HitResult Structure") (HitAnything :type Boolean))
  (bind _returnvalue (`Actor.K2_GetActorLocation` Skibidibi))
  (bind (_outhits _returnvalue_2) (`KismetSystemLibrary.SphereTraceMultiForObjects` _returnvalue (+ _returnvalue (* (`Actor.GetActorForwardVector` Skibidibi) (`self.SphereRadius`))) (`self.Radius`) (`self.DesiredObjects`) false (`self.Actors to Ignore`) (`self.DebugDraw`)))
  (return _outhits _returnvalue_2))

(fn `VisibilityTest`
  (params (Skibidibi :type "Pawn Object Reference") (`Hit Bot` :type "Actor Object Reference"))
  (returns (Success :type Boolean))
  (bind _outhit (`KismetSystemLibrary.LineTraceSingle` (`Actor.K2_GetActorLocation` Skibidibi) (`Actor.K2_GetActorLocation` `Hit Bot`) "TraceTypeQuery2" false (`self.Actors to Ignore`) (`self.DebugDraw`)))
  (if (== `Hit Bot` (`.HitActor` (`GameplayStatics.BreakHitResult` _outhit)))
    (bind _isfacingtarget (`self.IsFacingTarget` Skibidibi `Hit Bot`))
    (return _isfacingtarget)
    (else
      (return false))))